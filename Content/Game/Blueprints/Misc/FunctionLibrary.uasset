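; Blueprint function library with global helpers for player access and end-of-level screens.
; GetStyxCharacter returns player 0's pawn cast to StyxCharacter_BP.
; ForceGameOver and ForceLevelSuccess create their GameOver_WG or LevelSuccess_WG widget, add it to the viewport, switch player 0 to UI-only input and show the mouse cursor.
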(fn GetStyxCharacter
  (bind _asstyx_character_bp (Utilities|Casting|CastToStyxCharacter_BP (Game|GetPlayerCharacter 0)))
  (return _asstyx_character_bp))

(fn ForceGameOver
  (bind _returnvalue (Game|GetPlayerController 0))
  (bind _returnvalue_2 (UserInterface|CreateWidget "/Game/Game/Blueprints/UI/GameOver_WG.GameOver_WG_C" _returnvalue))
  (UserInterface|Viewport|AddtoViewport _returnvalue_2 0)
  (Input|SetInputModeUIOnly _returnvalue _returnvalue_2 "DoNotLock")
  (Variables|/Script/Engine.PlayerController|SetbShowMouseCursor _returnvalue true)
  (return))

(fn ForceLevelSuccess
  (bind _returnvalue (Game|GetPlayerController 0))
  (bind _returnvalue_2 (UserInterface|CreateWidget "/Game/Game/Blueprints/UI/LevelSuccess_WG.LevelSuccess_WG_C" _returnvalue))
  (UserInterface|Viewport|AddtoViewport _returnvalue_2 0)
  (Input|SetInputModeUIOnly _returnvalue _returnvalue_2 "DoNotLock")
  (Variables|/Script/Engine.PlayerController|SetbShowMouseCursor _returnvalue true)
  (return))