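; Hideout trigger volume that switches the view mode of the Styx character as it enters and leaves.
; Beginning overlap with the collider calls the character's switch-view event with the hideout view.
; Ending overlap scans every hideout volume for player 0, and only switches to the other view when none still overlaps, so adjacent or overlapping volumes act as one hideout.
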(event OnComponentBeginOverlap(HideOutCollider)
  (params (OverlappedComponent :type Primitive%20Component%20Object%20Reference) (OtherActor :type Actor%20Object%20Reference) (OtherComp :type Primitive%20Component%20Object%20Reference) (OtherBodyIndex :type Integer) (bFromSweep :type Boolean) (SweepResult :type Hit%20Result%20Structure%20%28by%20ref%29))
  (bind _asstyx_character_bp (Utilities|Casting|CastToStyxCharacter_BP OtherActor))
  (Default|OnSwitchViewEvent _asstyx_character_bp "NewEnumerator0"))

(event OnComponentEndOverlap(HideOutCollider)
  (params (OverlappedComponent :type Primitive%20Component%20Object%20Reference) (OtherActor :type Actor%20Object%20Reference) (OtherComp :type Primitive%20Component%20Object%20Reference) (OtherBodyIndex :type Integer))
  (Utilities|Array|Clear (Variables|Default|GetStyxHideouts))
  (bind _outactors (Actor|GetAllActorsOfClass "Styx_HideoutVolume_C"))
  (for _array_element _outactors
    (if (Collision|IsOverlappingActor (Variables|Styx_HideoutVolume_C|GetHideOutCollider _array_element) (Game|GetPlayerCharacter 0) :!class /Script/Engine.PrimitiveComponent)
      (Utilities|Array|Add (Variables|Default|GetStyxHideouts) _array_element)))
  (Variables|Default|SetbIsInHideout (select (> (Utilities|Array|Length (Variables|Default|GetStyxHideouts)) 0) true false))
  (if (not (Variables|Default|GetbIsInHideout))
    (bind _asstyx_character_bp (Utilities|Casting|CastToStyxCharacter_BP OtherActor))
    (Default|OnSwitchViewEvent _asstyx_character_bp "NewEnumerator1")))

(fn ConstructionScript)