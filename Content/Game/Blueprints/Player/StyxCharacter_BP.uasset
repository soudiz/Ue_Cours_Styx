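; Player character Blueprint with first/third-person camera switching, stamina-based movement, health and HUD-driven interactions.
; Run, jump, double jump and forward charge launch spend stamina; running interpolates walk speed and locks out when exhausted until stamina regenerates.
; Crouch resizes the capsule by timeline, with an upward sphere trace gating uncrouch.
; Tick feeds health and stamina to the HUD, interaction inputs notify CurrentIO, and zero health disables input.
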(event Custom|OnSwitchView_Event
  (params (NewView :type ViewMode_Enum%20Enum :default "NewEnumerator0"))
  (if (Variables|Controller|GetCanSwitchView)
    (Styx|SwitchViewFunction NewView)))

(event Custom|Regen%20Health%20Event
  (params (Health :type Float%20%28single-precision%29))
  (bind _output_get (Variables|PlayerState|SetHealth (Math|Float|Clamp(Float) (+ (Variables|PlayerState|GetHealth) Health) 0.0 1e+02)))
  (Math|Float|CompareFloat _output_get 0.0
    (:>
      _)
    (:==
      _))
  (Input|EnableInput (Game|GetPlayerController 0))
  (Variables|PlayerState|SetIsDead false))

(event Custom|Crouch%20Event
  (bind _mesh (Variables|Character|GetMesh))
  (bind _relativelocation (Variables|/Script/Engine.SceneComponent|GetRelativeLocation _mesh))
  (if (Variables|Controller|GetIsCrouching)
    (if (Variables|Controller|GetCanUnCrouch)
      (if (AI|Components|NavMovement|IsMovingonGround (Variables|Character|GetCharacterMovement))
        (Variables|Controller|SetIsCrouching false)
        (bind (_direction _lerpalpha) (Timeline|Timeline_0 Reverse)
          (:Update
            (Components|Capsule|SetCapsuleHalfHeight (Variables|Collision|GetCapsuleComponent) (Math|Float|Lerp (Variables|Controller|GetInitialHalfHeight) (Variables|Controller|GetCrouchHalfHeight) _lerpalpha) false)
            (Transformation|SetRelativeLocation _mesh (Math|Vector|MakeVector (.x _relativelocation) (.y _relativelocation) (* (Variables|/Script/Engine.CapsuleComponent|GetCapsuleHalfHeight (Variables|Collision|GetCapsuleComponent)) -1.0)) false false))
          (:Finished
            (switch Utilities|FlowControl|Switch|SwitchonETimelineDirection _direction
              (:Backward
                (Variables|/Script/Engine.CharacterMovementComponent|SetbCrouchMaintainsBaseLocation (Variables|Character|GetCharacterMovement) false)))))))
    (elif (AI|Components|NavMovement|IsMovingonGround (Variables|Character|GetCharacterMovement))
      (Variables|Controller|SetIsCrouching true)
      (Variables|/Script/Engine.CharacterMovementComponent|SetbCrouchMaintainsBaseLocation (Variables|Character|GetCharacterMovement) true)
      (Timeline|Timeline_0 Play))))

(event Custom|Charge%20Event
  (Character|LaunchCharacter (* (Transformation|GetActorForwardVector) (Variables|Controller|GetChargeForce)) true true)
  (Variables|PlayerState|SetStamina (Math|Float|Clamp(Float) (- (Variables|PlayerState|GetStamina) (Variables|Controller|GetChargeDecay)) 0.0 1e+02)))

(event EventTick
  (params (DeltaSeconds :type Float%20%28single-precision%29))
  (Utilities|FlowControl|Sequence
    (:then_0
      (Variables|Controller|SetCurrentHorizontalSpeed (Math|Vector|VectorLength (Math|Vector|ProjectVectorontoPlane (Transformation|GetVelocity) "0, 0,1.000000"))))
    (:then_1
      (if (Variables|Controller|GetIsCrouching)
        (bind _blocked (Styx|TestUncrouch))
        (Variables|Controller|SetCanUnCrouch (not _blocked))))
    (:then_2
      (if (Utilities|IsValid (Variables|UI|GetPlayerWidget))
        (Default|UpdateHealth (Variables|UI|GetPlayerWidget) (Variables|PlayerState|GetHealth) 1e+02)
        (Default|UpdateStamina (Variables|UI|GetPlayerWidget) (Variables|PlayerState|GetStamina) 1e+02)))))

(event EventBeginPlay
  (Variables|/Script/Engine.CharacterMovementComponent|SetMaxWalkSpeed (Variables|Character|GetCharacterMovement) (Variables|Controller|GetInitialWalkSpeed))
  (Variables|Controller|SetInitialHalfHeight (Components|Capsule|GetScaledCapsuleHalfHeight (Variables|Collision|GetCapsuleComponent)))
  (Variables|PlayerState|SetIsDead false)
  (Styx|SwitchViewFunction "NewEnumerator1")
  (EventDispatchers|BindEventtoOnSwitchView (delegate Custom|OnSwitchView_Event)))

(event EventOnLanded
  (params (Hit :type Hit%20Result%20Structure%20%28by%20ref%29))
  (Utilities|Time|ClearTimerbyFunctionName self "Charge Event"))

(event EventPossessed
  (params (NewController :type Controller%20Object%20Reference))
  (bind _returnvalue (UserInterface|CreateWidget "/Game/Game/Blueprints/UI/PlayerHUD_WG.PlayerHUD_WG_C"))
  (bind _output_get (Variables|UI|SetPlayerWidget _returnvalue))
  (Default|ShowHideDialText _output_get "Hidden")
  (Default|ShowHideInteraction _output_get "NewEnumerator7")
  (UserInterface|Viewport|AddtoViewport _output_get 0))

(event EventUnpossessed
  (params (OldController :type Controller%20Object%20Reference))
  (Utilities|IsValid (Variables|UI|GetPlayerWidget)
    (:Is%20Valid
      (Widget|RemovefromParent (Variables|UI|GetPlayerWidget)))))

(event Game|Damage|EventAnyDamage
  (params (Damage :type Float%20%28single-precision%29) (DamageType :type Damage%20Type%20Object%20Reference) (InstigatedBy :type Controller%20Object%20Reference) (DamageCauser :type Actor%20Object%20Reference))
  (bind _output_get (Variables|PlayerState|SetHealth (Math|Float|Clamp(Float) (- (Variables|PlayerState|GetHealth) Damage) 0.0 1e+02)))
  (Math|Float|CompareFloat _output_get 0.0
    (:==
      _)
    (:<
      _))
  (Input|DisableInput (Game|GetPlayerController 0))
  (Variables|PlayerState|SetIsDead true))

(event Input|ActionEvents|InputActionInteractionY
  (params (Key :type Key%20Structure :default "None"))
  (bind _currentio (Variables|Controller|GetCurrentIO))
  (:Pressed
    (if (and (Widget|IsVisible (Variables|/Game/Game/Blueprints/UI/PlayerHUD_WG.PlayerHUD_WG_C|GetInteractionY (Variables|UI|GetPlayerWidget))) (Utilities|IsValid _currentio))
      (Default|OnReceiveInteractionYEvent _currentio "NewEnumerator5"))))

(event Input|ActionEvents|InputActionInteractionX
  (params (Key :type Key%20Structure :default "None"))
  (bind _currentio (Variables|Controller|GetCurrentIO))
  (:Pressed
    (if (and (Widget|IsVisible (Variables|/Game/Game/Blueprints/UI/PlayerHUD_WG.PlayerHUD_WG_C|GetInteractionX (Variables|UI|GetPlayerWidget))) (Utilities|IsValid _currentio))
      (Default|OnReceiveInteractionXEvent _currentio "NewEnumerator4"))))

(event Input|ActionEvents|InputActionCrouch
  (params (Key :type Key%20Structure :default "None"))
  (:Pressed
    (CallFunction|CrouchEvent)))

(event Input|ActionEvents|InputActionInteractionB
  (params (Key :type Key%20Structure :default "None"))
  (bind _currentio (Variables|Controller|GetCurrentIO))
  (:Pressed
    (if (and (Widget|IsVisible (Variables|/Game/Game/Blueprints/UI/PlayerHUD_WG.PlayerHUD_WG_C|GetInteractionB (Variables|UI|GetPlayerWidget))) (Utilities|IsValid _currentio))
      (Default|OnReceiveInteractionBEvent _currentio "NewEnumerator6"))))

(event Input|ActionEvents|InputActionJump
  (params (Key :type Key%20Structure :default "None"))
  (:Pressed
    (if (AI|Components|NavMovement|IsMovingonGround (Variables|Character|GetCharacterMovement))
      (Character|Jump)
      (Variables|PlayerState|SetStamina (Math|Float|Clamp(Float) (- (Variables|PlayerState|GetStamina) (Variables|Controller|GetJumpDecay)) 0.0 1e+02) :!label _label)
      (elif (Variables|Controller|GetCanDoubleJump)
        (Character|LaunchCharacter (Math|Vector|MakeVector 0.0 0.0 (Variables|/Script/Engine.CharacterMovementComponent|GetJumpZVelocity (Variables|Character|GetCharacterMovement))) false true)
        (goto _label))))
  (:Released
    (Character|StopJumping)
    (Utilities|Time|ClearTimerbyFunctionName self "Charge Event")))

(event Input|AxisEvents|InputAxisLookUp
  (params (AxisValue :type Float%20%28single-precision%29))
  (Pawn|Input|AddControllerPitchInput AxisValue))

(event Input|AxisEvents|InputAxisTurn
  (params (AxisValue :type Float%20%28single-precision%29))
  (Pawn|Input|AddControllerYawInput AxisValue))

(event Input|AxisEvents|InputAxisTurnRate
  (params (AxisValue :type Float%20%28single-precision%29))
  (Pawn|Input|AddControllerYawInput (* AxisValue (Variables|Controller|GetBaseTurnRate) (Utilities|Time|GetWorldDeltaSeconds))))

(event Input|AxisEvents|InputAxisLookUpRate
  (params (AxisValue :type Float%20%28single-precision%29))
  (Pawn|Input|AddControllerPitchInput (* AxisValue (Variables|Controller|GetBaseLookUpRate) (Utilities|Time|GetWorldDeltaSeconds))))

(event Input|AxisEvents|InputAxisMoveForward
  (params (AxisValue :type Float%20%28single-precision%29))
  (Pawn|Input|AddMovementInput (Transformation|GetActorForwardVector) AxisValue false)
  (Variables|Controller|SetIsWalkingBackward (and (AI|Components|NavMovement|IsMovingonGround (Variables|Character|GetCharacterMovement)) (< AxisValue 0.0))))

(event Input|AxisEvents|InputAxisMoveRight
  (params (AxisValue :type Float%20%28single-precision%29))
  (Pawn|Input|AddMovementInput (Transformation|GetActorRightVector) AxisValue false)
  (Variables|Controller|SetIsStrafing (and (AI|Components|NavMovement|IsMovingonGround (Variables|Character|GetCharacterMovement)) (!= AxisValue 0.0))))

(event Input|AxisEvents|InputAxisRun
  (params (AxisValue :type Float%20%28single-precision%29))
  (if (!= AxisValue 0.0)
    (if (Math|Boolean|ANDBoolean (Variables|Controller|GetCanRun) (> (Variables|PlayerState|GetStamina) 0.1) (AI|Components|NavMovement|IsMovingonGround (Variables|Character|GetCharacterMovement)) (not (Variables|Controller|GetIsCrouching)) (not (Variables|Controller|GetIsStrafing)) (not (Variables|Controller|GetIsWalkingBackward)) (> (Variables|Controller|GetCurrentHorizontalSpeed) 1e+02))
      (Variables|Controller|SetIsRunning true)
      (bind _output_get (Variables|Controller|SetCurrentWalkSpeedSpeed (Math|Interpolation|FInterpTo (Variables|Controller|GetCurrentWalkSpeedSpeed) (Variables|Controller|GetRunningSpeed) (Utilities|Time|GetWorldDeltaSeconds) 5.0)))
      (Variables|/Script/Engine.CharacterMovementComponent|SetMaxWalkSpeed (Variables|Character|GetCharacterMovement) _output_get)
      (bind _output_get_2 (Variables|PlayerState|SetStamina (Math|Float|Clamp(Float) (- (Variables|PlayerState|GetStamina) (* (Variables|PlayerState|GetStaminaDecayRate) (Utilities|Time|GetWorldDeltaSeconds))) 0.0 1e+02)))
      (Math|Float|CompareFloat _output_get_2 0.0
        (:==
          _)
        (:<
          _))
      (Variables|Controller|SetCanRun false)
      (else
        (Variables|Controller|SetIsRunning false :!label _label)
        (bind _output_get_3 (Variables|Controller|SetCurrentWalkSpeedSpeed (Math|Interpolation|FInterpTo (Variables|Controller|GetCurrentWalkSpeedSpeed) (Variables|Controller|GetInitialWalkSpeed) (Utilities|Time|GetWorldDeltaSeconds) 5.0)))
        (Variables|/Script/Engine.CharacterMovementComponent|SetMaxWalkSpeed (Variables|Character|GetCharacterMovement) _output_get_3)
        (bind _output_get_4 (Variables|PlayerState|SetStamina (Math|Float|Clamp(Float) (+ (Variables|PlayerState|GetStamina) (* (Variables|PlayerState|GetStaminaRegenRate) (Utilities|Time|GetWorldDeltaSeconds))) 0.0 1e+02)))
        (Math|Float|CompareFloat _output_get_4 (Variables|PlayerState|GetMinStaminaToBeAbleToRunAgain)
          (:>
            _)
          (:==
            _))
        (Variables|Controller|SetCanRun true)))
    (else
      (goto _label))))

(fn ConstructionScript)

(fn TestUncrouch
  (bind _returnvalue (Transformation|GetActorLocation))
  (bind _capsulecomponent (Variables|Collision|GetCapsuleComponent))
  (bind _capsuleradius (Variables|/Script/Engine.CapsuleComponent|GetCapsuleRadius _capsulecomponent))
  (bind _returnvalue_2 (Collision|SphereTraceByChannel _returnvalue (+ _returnvalue (Math|Vector|MakeVector 0.0 0.0 (+ (Variables|/Script/Engine.CapsuleComponent|GetCapsuleHalfHeight _capsulecomponent) (/ _capsuleradius 2.0)))) (* _capsuleradius 0.75) "TraceTypeQuery1" true 0 "None"))
  (return _returnvalue_2))

(fn SwitchViewFunction
  (params (Selection :type ViewMode_Enum%20Enum :default "NewEnumerator0"))
  (bind _playerwidget (Variables|UI|GetPlayerWidget))
  (bind _playerwidget_2 (Variables|UI|GetPlayerWidget))
  (switch Utilities|FlowControl|Switch|SwitchonViewMode_Enum Selection
    (:NewEnumerator0
      (Variables|Controller|SetCurrentViewMode "NewEnumerator0")
      (Components|Activation|Deactivate (Variables|MyCharacter|GetTpsCamera))
      (Components|Activation|Activate (Variables|Default|GetFpsCamera) true)
      (Utilities|IsValid _playerwidget_2
        (:Is%20Valid
          (Default|ShowHideCrosshair _playerwidget_2 "Visible"))
        (:Is%20Not%20Valid
          _)))
    (:NewEnumerator1
      (Variables|Controller|SetCurrentViewMode "NewEnumerator1")
      (Components|Activation|Deactivate (Variables|Default|GetFpsCamera))
      (Components|Activation|Activate (Variables|MyCharacter|GetTpsCamera) true)
      (Utilities|IsValid _playerwidget
        (:Is%20Valid
          (Default|ShowHideCrosshair _playerwidget "Hidden"))
        (:Is%20Not%20Valid
          _))))
  (return))