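; MissionSheet is an objective actor that tracks one objective's state and shows it through an on-screen marker widget aimed at a target actor.
; Awake, Validate and Failed drive a guarded state machine (dormant to active, then validated or failed), each broadcasting a state change.
; Tick runs during the active state to refresh the marker text, and completion or failure removes the widget.
; StartAwake activates it at BeginPlay without broadcasting.
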(event EventBeginPlay
  (if (Variables|MissionObjective|GetStartAwake)
    (Actor|Tick|SetActorTickEnabled true)
    (DONOTUSE|ChangeObjectiveState "NewEnumerator1"))
  (bind _returnvalue (UserInterface|CreateWidget "/Game/Game/Blueprints/UI/ObjectiveMarker_WG.ObjectiveMarker_WG_C"))
  (Widget|SetVisibility _returnvalue (select (Variables|MissionObjective|GetStartAwake) "Visible" "Hidden"))
  (Variables|MissionObjective|SetObjectiveWidget _returnvalue)
  (Variables|/Game/Game/Blueprints/UI/ObjectiveMarker_WG.ObjectiveMarker_WG_C|SetObjectiveTarget _returnvalue (Variables|MissionObjective|GetObjectiveTargetActor))
  (UserInterface|Viewport|AddtoViewport _returnvalue 0))

(event EventTick
  (params (DeltaSeconds :type Float%20%28single-precision%29))
  (if (Utilities|Enum|Equal(Enum) (Variables|MissionObjective|GetObjectiveState) "NewEnumerator1")
    (Default|Update (Variables|MissionObjective|GetObjectiveWidget) (Variables|MissionObjective|GetObjectiveText))))

(fn ConstructionScript
  (Rendering|Components|TextRender|SetText (Variables|Default|GetTextRender) (Utilities|Text|ToText(String) (Utilities|GetDisplayName self))))

(fn ChangeObjectiveState
  (params (ObjectiveState :type EObjectiveState%20Enum :default "NewEnumerator0"))
  (Variables|MissionObjective|SetObjectiveState ObjectiveState)
  (return))

(fn Awake
  (if (Utilities|Enum|Equal(Enum) (Variables|MissionObjective|GetObjectiveState) "NewEnumerator0")
    (DONOTUSE|ChangeObjectiveState "NewEnumerator1")
    (Actor|Tick|SetActorTickEnabled true)
    (Default|CallOnStateChange "NewEnumerator1")
    (Widget|SetVisibility (Variables|MissionObjective|GetObjectiveWidget) "Visible")
    (return)))

(fn Validate
  (bind _objectivewidget (Variables|MissionObjective|GetObjectiveWidget))
  (if (Utilities|Enum|Equal(Enum) (Variables|MissionObjective|GetObjectiveState) "NewEnumerator1")
    (DONOTUSE|ChangeObjectiveState "NewEnumerator2")
    (Actor|Tick|SetActorTickEnabled false)
    (Default|CallOnStateChange "NewEnumerator2")
    (Widget|SetVisibility _objectivewidget "Hidden")
    (Widget|RemovefromParent _objectivewidget)
    (return)))

(fn Failed
  (bind _objectivewidget (Variables|MissionObjective|GetObjectiveWidget))
  (if (Utilities|Enum|Equal(Enum) (Variables|MissionObjective|GetObjectiveState) "NewEnumerator1")
    (DONOTUSE|ChangeObjectiveState "NewEnumerator3")
    (Actor|Tick|SetActorTickEnabled false)
    (Default|CallOnStateChange "NewEnumerator3")
    (Widget|SetVisibility _objectivewidget "Hidden")
    (Widget|RemovefromParent _objectivewidget)
    (return)))