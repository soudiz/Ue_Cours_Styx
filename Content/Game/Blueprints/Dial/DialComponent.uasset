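; Dialogue component that plays a sequence of text lines on the player's HUD.
; PlayDialogue_Event shows the dialogue text in the StyxCharacter_BP's PlayerWidget and steps through the passed array with a delayed manual loop.
; Each line stays up for its character count times TextSpeed, so longer lines display longer.
; After the last line it hides the text and calls OnDialEnded.
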(event Custom|PlayDialogue_Event
  (params (InText :type Array%20of%20Texts))
  (Variables|Default|SetIndexLoop 0)
  (bind _asstyx_character_bp (Utilities|Casting|CastToStyxCharacter_BP (Game|GetPlayerCharacter 0)))
  (Default|ShowHideDialText (Variables|/Game/Game/Blueprints/Player/StyxCharacter_BP.StyxCharacter_BP_C|GetPlayerWidget _asstyx_character_bp) "Visible")
  (if (< (Variables|Default|GetIndexLoop) (Utilities|Array|Length InText)) :!label _label
    (Rendering|Components|TextRender|SetText (Variables|/Game/Game/Blueprints/UI/PlayerHUD_WG.PlayerHUD_WG_C|GetDialText (Variables|/Game/Game/Blueprints/Player/StyxCharacter_BP.StyxCharacter_BP_C|GetPlayerWidget _asstyx_character_bp)) (Utilities|Array|Get(acopy) InText (Variables|Default|GetIndexLoop)))
    (Utilities|FlowControl|Delay (* (Utilities|String|Len (Utilities|String|ToString(Text) (Utilities|Array|Get(acopy) InText (Variables|Default|GetIndexLoop)))) (Variables|Default|GetTextSpeed)))
    (Math|Integer|IncrementInt (Variables|Default|GetIndexLoop)
      (:%20%20
        (goto _label)))
    (else
      (Default|ShowHideDialText (Variables|/Game/Game/Blueprints/Player/StyxCharacter_BP.StyxCharacter_BP_C|GetPlayerWidget _asstyx_character_bp) "Hidden")
      (Default|CallOnDialEnded))))