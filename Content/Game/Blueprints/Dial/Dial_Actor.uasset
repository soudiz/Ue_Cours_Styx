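; Dial_Actor is a placeable dialogue actor that plays a set of texts through its DialComponent.
; PlayDialogue_Event passes TextsToPlay to the component.
; The component's OnDialEnded is bound on BeginPlay and re-broadcast through the actor's own OnDialEnded dispatcher.
; The construction script labels the actor by writing its display name to the DialName text in TextColor.
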(event Custom|PlayDialogue_Event
  (Default|PlayDialogueEvent (Variables|Default|GetDialComponent) (Variables|Dialogue|GetTextsToPlay)))

(event Custom|CustomEvent_OnDialEnded
  (Default|CallOnDialEnded))

(event EventBeginPlay
  (EventDispatchers|BindEventtoOnDialEnded (Variables|Default|GetDialComponent) (delegate Custom|CustomEvent_OnDialEnded)))

(fn ConstructionScript
  (bind _dialname (Variables|Default|GetDialName))
  (Rendering|Components|TextRender|SetText _dialname (Utilities|Text|ToText(String) (Utilities|GetDisplayName self)))
  (Rendering|Components|TextRender|SetTextRenderColor _dialname (Variables|Dialogue|GetTextColor)))