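; Base AI pawn that patrols through a behavior tree and can be killed or talked to by interaction.
; It runs BT_AI when given a starting patrol, and a StartPatrol event restarts the tree and sets a new patrol node.
; Two child interaction-object actors, toggled by killable and talkable flags, handle kill and talk.
; Talking plays a dialogue, disabling talk until it ends if repeatable; death and dialogue end are broadcast.
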(event Custom|OnUseEnded_Kill
  (params (InteractionUsed :type EInteractionAllowed%20Enum :default "NewEnumerator0"))
  (switch Utilities|FlowControl|Switch|SwitchonEInteractionAllowed InteractionUsed
    (:NewEnumerator4
      (if (Variables|AI|GetIsAlive)
        (Default|Kill (Variables|AI|GetIOKill) self)
        (Default|CallOnAiDied)))))

(event Custom|OnUseEnded_Talk
  (params (InteractionUsed :type EInteractionAllowed%20Enum :default "NewEnumerator0"))
  (bind _dialtoplay (Variables|AI|GetDialToPlay))
  (switch Utilities|FlowControl|Switch|SwitchonEInteractionAllowed InteractionUsed
    (:NewEnumerator5
      (Utilities|IsValid _dialtoplay
        (:Is%20Valid
          (Default|PlayDialogueEvent _dialtoplay)
          (AI|SetIsTalkable false)
          (EventDispatchers|AssignOnDialEnded _dialtoplay (delegate Custom|OnDialEnded_Event_0)))))))

(event Custom|StartPatrol_Event
  (params (PatrolPoint :type AI%20Patrol%20Node%20Object%20Reference))
  (bind _self self)
  (bind _returnvalue (AI|GetAIController _self))
  (bind _braincomponent (Variables|/Script/AIModule.AIController|GetBrainComponent _returnvalue))
  (if (Variables|AI|GetIsAlive)
    (Utilities|FlowControl|Sequence
      (:then_0
        (if (Class|BrainComponent|IsRunning _braincomponent)
          (AI|Logic|StopLogic _braincomponent "Patrol"))
        (AI|RunBehaviorTree _returnvalue "/Game/Game/Blueprints/AI/BT_AI.BT_AI"))
      (:then_1
        (Variables|Patrol|SetCurrentPatrolNode PatrolPoint)))))

(event Custom|OnDialEnded_Event_0
  (if (Variables|AI|GetTalkableMultipleTimes)
    (AI|SetIsTalkable true))
  (Default|CallOnAiTalkEnded (Variables|AI|GetDialToPlay)))

(event EventBeginPlay
  (Utilities|FlowControl|Sequence
    (:then_0
      (Utilities|IsValid (Variables|Patrol|GetStartingPatrol)
        (:Is%20Valid
          (AI|RunBehaviorTree (AI|GetAIController self) "/Game/Game/Blueprints/AI/BT_AI.BT_AI"))))
    (:then_1
      (EventDispatchers|BindEventtoStartPatrol (delegate Custom|StartPatrol_Event)))
    (:then_2
      (bind _asai_iokill (Utilities|Casting|CastToAI_IOKill (Variables|/Script/Engine.ChildActorComponent|GetChildActor (Variables|Default|GetChild_IOKill))))
      (Variables|AI|SetIOKill _asai_iokill))
    (:then_3
      (bind _asai_iotalk (Utilities|Casting|CastToAI_IOTalk (Variables|/Script/Engine.ChildActorComponent|GetChildActor (Variables|Default|GetChild_IOTalk))))
      (Variables|AI|SetIOTalk _asai_iotalk))
    (:then_4
      (if (not (Variables|AI|GetIsKillable))
        (Default|ChangeIOState (Variables|AI|GetIOKill) false)))
    (:then_5
      (if (not (Variables|AI|GetIsTalkable))
        (Default|ChangeIOState (Variables|AI|GetIOTalk) false)))
    (:then_6
      (EventDispatchers|AssignOnUseEnded (Variables|AI|GetIOKill) (delegate Custom|OnUseEnded_Kill)))
    (:then_7
      (EventDispatchers|AssignOnUseEnded (Variables|AI|GetIOTalk) (delegate Custom|OnUseEnded_Talk)))))

(fn ConstructionScript
  (bind _startingpatrol (Variables|Patrol|GetStartingPatrol))
  (|CallParentFunction)
  (Utilities|IsValid _startingpatrol
    (:Is%20Valid
      (Variables|Patrol|SetCurrentPatrolNode _startingpatrol))
    (:Is%20Not%20Valid
      (Variables|Patrol|SetCurrentPatrolNode 0))))

(fn KillAi
  (bind _asai_iokill (Utilities|Casting|CastToAI_IOKill (Variables|/Script/Engine.ChildActorComponent|GetChildActor (Variables|Default|GetChild_IOKill))))
  (Default|Kill _asai_iokill self))

(fn SetIsKillable
  (if (not (Variables|AI|GetIsKillable))
    (Default|ChangeIOState (Variables|AI|GetIOKill) true)
    (Variables|AI|SetIsKillable true)
    (return)))

(fn SetIsTalkable
  (params (IsTalkable :type Boolean))
  (Variables|AI|SetIsTalkable IsTalkable)
  (Default|ChangeIOState (Variables|AI|GetIOTalk) IsTalkable)
  (return))