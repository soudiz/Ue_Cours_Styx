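; AI_PatrolNode is a patrol waypoint Blueprint whose construction script links it to a NextPoint and visualizes the route.
; When NextPoint is valid, it copies its own PreviousPoint reference into that node's PreviousPoint and snaps its spline's second point to that node's location.
; An arrow component is visible only when WaitTime is positive or exactly -1, marking nodes with a wait.
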(fn ConstructionScript
  (bind _nextpoint (Variables|Patrol|GetNextPoint))
  (bind _waittime (Variables|Patrol|GetWaitTime))
  (Utilities|FlowControl|Sequence
    (:then_0
      (Utilities|IsValid _nextpoint
        (:Is%20Valid
          (Variables|AI_PatrolNode_C|SetPreviousPoint _nextpoint (Variables|Patrol|GetPreviousPoint))
          (Spline|SetLocationatSplinePoint (Variables|Default|GetSpline) 1 (Transformation|GetActorLocation _nextpoint) "World" true))))
    (:then_1
      (Rendering|SetVisibility (Variables|Default|GetArrow) (or (> _waittime 0.0) (== _waittime -1.0)) false))))