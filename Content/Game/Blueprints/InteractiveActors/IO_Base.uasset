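; Base interactive object that registers itself with the Styx character and drives the Y, X and B interaction prompts.
; While enabled, Box overlap sets the character's CurrentIO and fills the player widget, and leaving clears both.
; Y, X and B interaction events call OnUseEnded, then disable single-use objects.
; ChangeIOState toggles state and Box collision, then updates the player's registration and prompt.
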(event OnComponentBeginOverlap(Box)
  (params (OverlappedComponent :type Primitive%20Component%20Object%20Reference) (OtherActor :type Actor%20Object%20Reference) (OtherComp :type Primitive%20Component%20Object%20Reference) (OtherBodyIndex :type Integer) (bFromSweep :type Boolean) (SweepResult :type Hit%20Result%20Structure%20%28by%20ref%29))
  (switch Utilities|FlowControl|Switch|SwitchonEInteractiveActorsState (Variables|InteractiveActors|GetIO_State)
    (:NewEnumerator0
      (bind _asstyx_character_bp (Utilities|Casting|CastToStyxCharacter_BP OtherActor))
      (Variables|/Game/Game/Blueprints/Player/StyxCharacter_BP.StyxCharacter_BP_C|SetCurrentIO _asstyx_character_bp self)
      (Default|ShowHideInteraction (Variables|/Game/Game/Blueprints/Player/StyxCharacter_BP.StyxCharacter_BP_C|GetPlayerWidget _asstyx_character_bp) (Variables|InteractiveActors|GetInteractionAllowed))
      (Rendering|Components|TextRender|SetText (Variables|/Game/Game/Blueprints/UI/PlayerHUD_WG.PlayerHUD_WG_C|GetText_InteractionY (Variables|/Game/Game/Blueprints/Player/StyxCharacter_BP.StyxCharacter_BP_C|GetPlayerWidget _asstyx_character_bp)) (Variables|InteractiveActors|GetInteractionTextY))
      (Rendering|Components|TextRender|SetText (Variables|/Game/Game/Blueprints/UI/PlayerHUD_WG.PlayerHUD_WG_C|GetText_InteractionX (Variables|/Game/Game/Blueprints/Player/StyxCharacter_BP.StyxCharacter_BP_C|GetPlayerWidget _asstyx_character_bp)) (Variables|InteractiveActors|GetInteractionTextX))
      (Rendering|Components|TextRender|SetText (Variables|/Game/Game/Blueprints/UI/PlayerHUD_WG.PlayerHUD_WG_C|GetText_InteractionB (Variables|/Game/Game/Blueprints/Player/StyxCharacter_BP.StyxCharacter_BP_C|GetPlayerWidget _asstyx_character_bp)) (Variables|InteractiveActors|GetInteractionTextB)))))

(event OnComponentEndOverlap(Box)
  (params (OverlappedComponent :type Primitive%20Component%20Object%20Reference) (OtherActor :type Actor%20Object%20Reference) (OtherComp :type Primitive%20Component%20Object%20Reference) (OtherBodyIndex :type Integer))
  (switch Utilities|FlowControl|Switch|SwitchonEInteractiveActorsState (Variables|InteractiveActors|GetIO_State)
    (:NewEnumerator0
      (InteractiveActors|DisablePlayerInput OtherActor))))

(event Custom|OnReceiveInteractionY_Event
  (params (InteractionUsed :type EInteractionAllowed%20Enum :default "NewEnumerator0"))
  (Default|CallOnUseEnded InteractionUsed)
  (if (not (Variables|InteractiveActors|GetCanBeUsedMultipleTimes))
    (InteractiveActors|ChangeIOState false)))

(event Custom|OnReceiveInteractionX_Event
  (params (InteractionUsed :type EInteractionAllowed%20Enum :default "NewEnumerator0"))
  (Default|CallOnUseEnded InteractionUsed)
  (if (not (Variables|InteractiveActors|GetCanBeUsedMultipleTimes))
    (InteractiveActors|ChangeIOState false)))

(event Custom|OnReceiveInteractionB_Event
  (params (InteractionUsed :type EInteractionAllowed%20Enum :default "NewEnumerator0"))
  (Default|CallOnUseEnded InteractionUsed)
  (if (not (Variables|InteractiveActors|GetCanBeUsedMultipleTimes))
    (InteractiveActors|ChangeIOState false)))

(fn ConstructionScript)

(fn ChangeIOState
  (params (Enable? :type Boolean))
  (Variables|InteractiveActors|SetIO_State (select Enable? "NewEnumerator0" "NewEnumerator1"))
  (Collision|SetCollisionEnabled (Variables|Default|GetBox) (select Enable? "QueryAndPhysics" "NoCollision"))
  (if Enable?
    (if (Collision|IsOverlappingActor self (CallFunction|GetStyxCharacter) :!class /Script/Engine.Actor)
      (InteractiveActors|EnablePlayerInput self))
    (else
      (InteractiveActors|DisablePlayerInput (Game|GetPlayerCharacter 0))))
  (return))

(fn DisablePlayerInput
  (params (EnteredCharacter :type Object%20Object%20Reference))
  (bind _asstyx_character_bp (Utilities|Casting|CastToStyxCharacter_BP EnteredCharacter))
  (Variables|/Game/Game/Blueprints/Player/StyxCharacter_BP.StyxCharacter_BP_C|SetCurrentIO _asstyx_character_bp 0)
  (Default|ShowHideInteraction (Variables|/Game/Game/Blueprints/Player/StyxCharacter_BP.StyxCharacter_BP_C|GetPlayerWidget _asstyx_character_bp) "NewEnumerator7"))

(fn EnablePlayerInput
  (params (NewCurrentIO :type IO%20Base%20Object%20Reference))
  (bind _asstyx_character_bp (Utilities|Casting|CastToStyxCharacter_BP (Game|GetPlayerCharacter 0)))
  (Variables|/Game/Game/Blueprints/Player/StyxCharacter_BP.StyxCharacter_BP_C|SetCurrentIO _asstyx_character_bp NewCurrentIO)
  (Default|ShowHideInteraction (Variables|/Game/Game/Blueprints/Player/StyxCharacter_BP.StyxCharacter_BP_C|GetPlayerWidget _asstyx_character_bp) (Variables|IO_Base_C|GetInteractionAllowed NewCurrentIO)))